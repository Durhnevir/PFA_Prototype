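; Player controller that rotates the player character's camera in quarter turns.
; The CamRotationRight and CamRotationLeft input actions cast the player character to Bp_Player and read its SpringArm1 world rotation.
; Each press instantly sets the spring arm yaw 90 degrees in opposite directions, keeping roll and pitch unchanged, with no interpolation.
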(event EventBeginPlay)

(event EventTick
  (params (DeltaSeconds :type Float%20%28single-precision%29)))

(event Input|ActionEvents|InputActionCamRotationLeft
  (params (Key :type Key%20Structure :default "None"))
  (:Pressed
    (bind _asbp_player (Utilities|Casting|CastToBp_Player (Game|GetPlayerCharacter 0)))
    (bind _output_get (Variables|Ressources|SetArmRotation (Math|Rotator|MakeRotator (.roll (Transformation|GetWorldRotation (Variables|/Game/Blueprint/Player/Bp_Player.Bp_Player_C|GetSpringArm1 _asbp_player))) (.pitch (Transformation|GetWorldRotation (Variables|/Game/Blueprint/Player/Bp_Player.Bp_Player_C|GetSpringArm1 _asbp_player))) (+ (.yaw (Transformation|GetWorldRotation (Variables|/Game/Blueprint/Player/Bp_Player.Bp_Player_C|GetSpringArm1 _asbp_player))) 9e+01))))
    (Transformation|SetWorldRotation (Variables|/Game/Blueprint/Player/Bp_Player.Bp_Player_C|GetSpringArm1 _asbp_player) _output_get false false)))

(event Input|ActionEvents|InputActionCamRotationRight
  (params (Key :type Key%20Structure :default "None"))
  (:Pressed
    (bind _asbp_player (Utilities|Casting|CastToBp_Player (Game|GetPlayerCharacter 0)))
    (bind _output_get (Variables|Ressources|SetArmRotation (Math|Rotator|MakeRotator (.roll (Transformation|GetWorldRotation (Variables|/Game/Blueprint/Player/Bp_Player.Bp_Player_C|GetSpringArm1 _asbp_player))) (.pitch (Transformation|GetWorldRotation (Variables|/Game/Blueprint/Player/Bp_Player.Bp_Player_C|GetSpringArm1 _asbp_player))) (+ (.yaw (Transformation|GetWorldRotation (Variables|/Game/Blueprint/Player/Bp_Player.Bp_Player_C|GetSpringArm1 _asbp_player))) -9e+01))))
    (Transformation|SetWorldRotation (Variables|/Game/Blueprint/Player/Bp_Player.Bp_Player_C|GetSpringArm1 _asbp_player) _output_get false false)))

(fn ConstructionScript)