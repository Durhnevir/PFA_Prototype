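; BP_CornerTrigger is a box trigger that appears meant to detect which side the player enters a corner from, but is currently inactive.
; BeginPlay caches the Bp_Player reference, while both overlap events are empty.
; Disconnected nodes dot the spring arm's right vector with the trigger-to-player direction to print left or right.
; Other unwired nodes toggle player input and set both controller rotation-check flags.
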(event OnComponentBeginOverlap(Box)
  (params (OverlappedComponent :type Primitive%20Component%20Object%20Reference) (OtherActor :type Actor%20Object%20Reference) (OtherComp :type Primitive%20Component%20Object%20Reference) (OtherBodyIndex :type Integer) (bFromSweep :type Boolean) (SweepResult :type Hit%20Result%20Structure%20%28by%20ref%29)))

(event OnComponentEndOverlap(Box)
  (params (OverlappedComponent :type Primitive%20Component%20Object%20Reference) (OtherActor :type Actor%20Object%20Reference) (OtherComp :type Primitive%20Component%20Object%20Reference) (OtherBodyIndex :type Integer)))

(event EventBeginPlay
  ;[1 1 1] Calcule le dot entre foward vecteur du trigger et du player > Pour savoir par quel face la player entre dans le trigger
  (bind _asbp_player (Utilities|Casting|CastToBp_Player (Game|GetPlayerCharacter 0))))

(fn ConstructionScript)