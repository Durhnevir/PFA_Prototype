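; Parent Blueprint for island ("Ile") actors that register with BP_Focus and can rotate in quarter turns.
; BeginPlay caches the box's bottom Z as Hauteur and finds BP_Focus.
; Box overlaps pass the box's owner to BP_Focus and call GetFocusedIle.
; Left/right rotation swaps and negates world X/Y, orbiting the world origin, and yaws 90 degrees; focus-relative sign checks feed identical branches, so have no effect.
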(event OnComponentBeginOverlap(Box)
  (params (OverlappedComponent :type Primitive%20Component%20Object%20Reference) (OtherActor :type Actor%20Object%20Reference) (OtherComp :type Primitive%20Component%20Object%20Reference) (OtherBodyIndex :type Integer) (bFromSweep :type Boolean) (SweepResult :type Hit%20Result%20Structure%20%28by%20ref%29))
  (bind _focusref (Variables|Ressources|GetFocusRef))
  (Variables|/Game/Blueprint/OtherBP/BP_Focus.BP_Focus_C|SetOverlapedIleRef _focusref (Components|GetOwner OverlappedComponent))
  (Default|GetFocusedIle _focusref))

(event EventBeginPlay
  (CallFunction|GetIleHight)
  (bind _returnvalue (Actor|GetActorOfClass "/Game/Blueprint/OtherBP/BP_Focus.BP_Focus_C"))
  (Variables|Ressources|SetFocusRef _returnvalue))

(fn ConstructionScript)

(fn GetIleHight
  (bind _box (Variables|Default|GetBox))
  (Variables|Ressources|SetHauteur (- (.z (Transformation|GetWorldLocation _box)) (.z (Variables|/Script/Engine.BoxComponent|GetBoxExtent _box)))))

(fn SetIleRightRotation
  (bind _scene (Variables|Default|GetScene))
  (bind _scene_2 (Variables|Default|GetScene))
  (bind _scene_3 (Variables|Default|GetScene))
  (bind _scene_4 (Variables|Default|GetScene))
  (bind _scene_5 (Variables|Default|GetScene))
  (bind _returnvalue (Transformation|GetWorldLocation _scene))
  (bind _returnvalue_2 (Transformation|GetWorldLocation _scene_2))
  (bind _returnvalue_3 (Transformation|GetWorldLocation _scene_4))
  (bind _returnvalue_4 (Transformation|GetWorldLocation _scene_5))
  (bind _returnvalue_5 (Transformation|GetWorldRotation _scene_3))
  (Variables|Ressources|SetFocus>IleVector (- (Transformation|GetWorldLocation (Variables|Default|GetScene)) (Transformation|GetWorldLocation (Variables|/Game/Blueprint/OtherBP/BP_Focus.BP_Focus_C|GetDefaultSceneRoot (Variables|Ressources|GetFocusRef)))))
  (Utilities|FlowControl|Sequence
    (:then_0
      (Math|Float|CompareFloat (.x (Variables|Ressources|GetFocus>IleVector)) 0.0
        (:>
          (Variables|Ressources|SetPositiveX true))
        (:<
          (Variables|Ressources|SetPositiveX false))))
    (:then_1
      (Math|Float|CompareFloat (.y (Variables|Ressources|GetFocus>IleVector)) 0.0
        (:>
          (Variables|Ressources|SetPositiveY true))
        (:<
          (Variables|Ressources|SetPositiveY false))))
    (:then_2
      (if (Variables|Ressources|GetPositiveX)
        (if (Variables|Ressources|GetPositiveY)
          (Transformation|SetWorldLocation _scene_5 (Math|Vector|MakeVector (.y _returnvalue_4) (* (.x _returnvalue_4) -1.0) (.z _returnvalue_4)) false false)
          (else
            (Transformation|SetWorldLocation _scene (Math|Vector|MakeVector (.y _returnvalue) (* (.x _returnvalue) -1.0) (.z _returnvalue)) false false)))
        (elif (Variables|Ressources|GetPositiveY)
          (Transformation|SetWorldLocation _scene_4 (Math|Vector|MakeVector (.y _returnvalue_3) (* (.x _returnvalue_3) -1.0) (.z _returnvalue_3)) false false)
          (else
            (Transformation|SetWorldLocation _scene_2 (Math|Vector|MakeVector (.y _returnvalue_2) (* (.x _returnvalue_2) -1.0) (.z _returnvalue_2)) false false)))))
    (:then_3
      (Transformation|SetWorldRotation _scene_3 (Math|Rotator|MakeRotator (.roll _returnvalue_5) (.pitch _returnvalue_5) (- (.yaw _returnvalue_5) 9e+01)) false false))))

(fn SetIleLeftRotation
  (bind _scene (Variables|Default|GetScene))
  (bind _scene_2 (Variables|Default|GetScene))
  (bind _scene_3 (Variables|Default|GetScene))
  (bind _scene_4 (Variables|Default|GetScene))
  (bind _scene_5 (Variables|Default|GetScene))
  (bind _returnvalue (Transformation|GetWorldLocation _scene))
  (bind _returnvalue_2 (Transformation|GetWorldLocation _scene_5))
  (bind _returnvalue_3 (Transformation|GetWorldLocation _scene_2))
  (bind _returnvalue_4 (Transformation|GetWorldLocation _scene_4))
  (bind _returnvalue_5 (Transformation|GetWorldRotation _scene_3))
  (Variables|Ressources|SetFocus>IleVector (- (Transformation|GetWorldLocation (Variables|Default|GetScene)) (Transformation|GetWorldLocation (Variables|/Game/Blueprint/OtherBP/BP_Focus.BP_Focus_C|GetDefaultSceneRoot (Variables|Ressources|GetFocusRef)))))
  (Utilities|FlowControl|Sequence
    (:then_0
      (Math|Float|CompareFloat (.x (Variables|Ressources|GetFocus>IleVector)) 0.0
        (:>
          (Variables|Ressources|SetPositiveX true))
        (:<
          (Variables|Ressources|SetPositiveX false))))
    (:then_1
      (Math|Float|CompareFloat (.y (Variables|Ressources|GetFocus>IleVector)) 0.0
        (:>
          (Variables|Ressources|SetPositiveY true))
        (:<
          (Variables|Ressources|SetPositiveY false))))
    (:then_2
      (if (Variables|Ressources|GetPositiveX)
        (if (Variables|Ressources|GetPositiveY)
          (Transformation|SetWorldLocation _scene_5 (Math|Vector|MakeVector (* (.y _returnvalue_2) -1.0) (.x _returnvalue_2) (.z _returnvalue_2)) false false)
          (else
            (Transformation|SetWorldLocation _scene (Math|Vector|MakeVector (* (.y _returnvalue) -1.0) (.x _returnvalue) (.z _returnvalue)) false false)))
        (elif (Variables|Ressources|GetPositiveY)
          (Transformation|SetWorldLocation _scene_4 (Math|Vector|MakeVector (* (.y _returnvalue_4) -1.0) (.x _returnvalue_4) (.z _returnvalue_4)) false false)
          (else
            (Transformation|SetWorldLocation _scene_2 (Math|Vector|MakeVector (* (.y _returnvalue_3) -1.0) (.x _returnvalue_3) (.z _returnvalue_3)) false false)))))
    (:then_3
      (Transformation|SetWorldRotation _scene_3 (Math|Rotator|MakeRotator (.roll _returnvalue_5) (.pitch _returnvalue_5) (+ (.yaw _returnvalue_5) 9e+01)) false false))))