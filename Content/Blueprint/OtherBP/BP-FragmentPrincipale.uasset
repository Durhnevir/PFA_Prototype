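; BP-FragmentPrincipale is a child fragment Blueprint, apparently the main fragment, that adds an EndLevel counter to its parent's behavior.
; BeginPlay runs the parent logic, then resets EndLevel to zero.
; DestroyFragment calls the parent implementation, then increments EndLevel.
; Both events print the counter for debugging; nothing in this Blueprint acts on its value, and overlap and Tick are disabled stubs.
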(event EventBeginPlay
  (|CallParentFunction)
  (bind _output_get (Variables|Default|SetEndLevel 0))
  (Development|PrintString (Utilities|String|ToString(Integer) _output_get)))

(event Collision|EventActorBeginOverlap
  (params (OtherActor :type Actor%20Object%20Reference))
  (|CallParentFunction OtherActor) ; This node is disabled and will not be called.\nDrag off pins to build functionality.
)

(event EventTick
  (params (DeltaSeconds :type Float%20%28single-precision%29))
  (|CallParentFunction DeltaSeconds) ; This node is disabled and will not be called.\nDrag off pins to build functionality.
)

(event EventDestroyFragment
  (|CallParentFunction)
  (bind _output_get (Variables|Default|SetEndLevel (+ (Variables|Default|GetEndLevel) 1)))
  (Development|PrintString (Utilities|String|ToString(Integer) _output_get)))

(fn ConstructionScript
  (|CallParentFunction))